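; HeatwaveGameMode is the game mode for Heatwave and provides the entry point for rotating the sun.
; On BeginPlay it casts the game state to HeatwaveGameState and caches the reference.
; RotateSunTo uses that reference to call ShineAllTiles on the field, then rotates the sun to the new direction.
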(event EventBeginPlay
  (CallFunction|LinkGameState))

(fn ConstructionScript)

(fn RotateSunto
  (params (newDirection :type Direction%20Enum :default "NewEnumerator0"))
  (Default|ShineAllTiles (Default|GetField (Variables|Default|GetgameStateRef)))
  (Default|Rotateto (Default|GetSun (Variables|Default|GetgameStateRef)) newDirection))

(fn LinkGameState
  (bind _asheatwave_game_state (Utilities|Casting|CastToHeatwaveGameState (Game|GetGameState)))
  (Variables|Default|SetgameStateRef _asheatwave_game_state))