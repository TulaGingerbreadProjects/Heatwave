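; MenuHUD is a menu HUD Blueprint with functions for main, levels, settings, pause and exit menus, mostly placeholders.
; Each handler prints a debug string, and only Exit does more by quitting the game.
; OpenMenu currently just returns true; its switch on MenuType that would route MenuCommand to the handlers is disconnected and never runs.
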(fn ConstructionScript)

(fn OpenMenu
  (params (menuCommand :type Menu%20Command%20Object%20Reference))
  ;[1 1 1] TODO: any improvements?
  (return true))

(fn OpenSettings
  (params (menuCommand :type Menu%20Command%20Object%20Reference))
  (Development|PrintString "Open settings menu"))

(fn OpenLevels
  (params (menuCommand :type Menu%20Command%20Object%20Reference))
  (Development|PrintString "Open level selection menu"))

(fn Exit
  (params (menuCommand :type Menu%20Command%20Object%20Reference))
  (Development|PrintString "Quit game")
  (Game|QuitGame 0 "Quit" false))

(fn OpenPauseMenu
  (params (menuCommand :type Menu%20Command%20Object%20Reference))
  (Development|PrintString "Open pause menu"))

(fn OpenMainMenu
  (params (menuCommand :type Menu%20Command%20Object%20Reference))
  (Development|PrintString "Open main menu")
  (return))