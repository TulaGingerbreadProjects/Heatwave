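; HeatwaveGameState is a game state Blueprint that serves as a shared access point for the level's Sun and Field actors.
; On BeginPlay it finds the first actor of each class with GetAllActorsOfClass and caches the references.
; The getters lazily re-link when a cached reference is invalid, and setters allow either reference to be replaced.
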(event EventBeginPlay
  ;[0 0.5 0] Perfect
  (Sun|LinkSun)
  (Field|LinkField))

(fn ConstructionScript)

(fn LinkSun
  ;[0 0.5 0] Perfect
  (bind _outactors (Actor|GetAllActorsOfClass "/Game/Blueprints/Sun/Sun.Sun_C"))
  (Variables|References|SetsunRef (Utilities|Array|Get(acopy) _outactors)))

(fn LinkField
  ;[0 0.5 0] Perfect
  (bind _outactors (Actor|GetAllActorsOfClass "/Game/Blueprints/Field/Field.Field_C"))
  (Variables|References|SetfieldRef (Utilities|Array|Get(acopy) _outactors)))

(fn GetSun
  ;[0 0.5 0] Perfect
  (Utilities|IsValid (Variables|References|GetsunRef)
    (:Is%20Valid
      _)
    (:Is%20Not%20Valid
      (Sun|LinkSun)))
  (return (Variables|References|GetsunRef)))

(fn SetSun
  (params (newSun :type Sun%20Object%20Reference))
  ;[0 0.5 0] Perfect
  (Variables|References|SetsunRef newSun))

(fn GetField
  ;[0 0.5 0] Perfect
  (Utilities|IsValid (Variables|References|GetfieldRef)
    (:Is%20Valid
      _)
    (:Is%20Not%20Valid
      (Field|LinkField)))
  (return (Variables|References|GetfieldRef)))

(fn SetField
  (params (newField :type Field%20Object%20Reference))
  ;[0 0.5 0] Perfect
  (Variables|References|SetfieldRef newField))