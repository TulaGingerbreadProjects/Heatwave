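; Player controller for a tile game where the player traces a path of neighboring tiles to move the pawn.
; While SelectTile or F is held, ProceedSelectedTile queues tiles adjacent to the path's end, or the current tile if empty, and backtracking onto the second-to-last tile removes the last.
; On release, the pawn jumps to the last tile, the game quits if the path contains the field's FinishTile, and the queue clears.
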(event Input|ActionEvents|InputActionSelectTile
  (params (Key :type Key%20Structure))
  (:Pressed
    (Variables|Default|SetisSelecting true))
  (:Released
    (Variables|Default|SetisSelecting false)
    (CallFunction|MoveCharactertoPosition)
    (Utility|ClearQueue)))

(event Input|KeyboardEvents|F
  (params (Key :type Key%20Structure))
  (:Pressed
    (Variables|Default|SetisSelecting true))
  (:Released
    (Variables|Default|SetisSelecting false)
    (CallFunction|MoveCharactertoPosition)
    (Utility|ClearQueue)))

(fn ConstructionScript)

(fn AddTileifNeighbor
  (params (tileRef :type Tile%20Object%20Reference))
  (if (Default|IsNeighbor tileRef (select (Utility|IsQueueEmpty) (Variables|Default|GetcurrentTile) (SpecificTiles|GetLastTile))) ; TODO: REPLACE WITH SELECT
    (CallFunction|AddTiletoQueue tileRef :!label _label)
    (elif (Default|IsNeighbor tileRef (SpecificTiles|GetLastTile))
      (goto _label))))

(fn ClearQueue
  (for _array_element (Variables|Default|GettilesQueue)
    (Default|DiscardTile _array_element))
  (Utilities|Array|Clear (Variables|Default|GettilesQueue)))

(fn ProceedSelectedTile
  (params (tileRef :type Tile%20Object%20Reference))
  (if (Variables|Default|GetisSelecting)
    (if (Default|IsSelected tileRef)
      (CallFunction|RemoveifReverse tileRef)
      (else
        (CallFunction|AddTileifNeighbor tileRef)))))

(fn IsLastTile
  (params (tileRef :type Tile%20Object%20Reference))
  (return (== tileRef (SpecificTiles|GetLastTile))))

(fn RemoveTilefromQueue
  (params (tileRef :type Tile%20Object%20Reference))
  (Utilities|Array|RemoveItem (Variables|Default|GettilesQueue) tileRef)
  (Default|DiscardTile tileRef))

(fn RemoveifReverse
  (params (tileRef :type Tile%20Object%20Reference))
  (if (SpecificTiles|IsPenultTile tileRef)
    (CallFunction|RemoveTilefromQueue (SpecificTiles|GetLastTile))))

(fn IsQueueEmpty
  (return (== (Utilities|Array|Length (Variables|Default|GettilesQueue)) 0)))

(fn GetLastTile
  (bind _tilesqueue (Variables|Default|GettilesQueue))
  (if (Utility|IsQueueEmpty)
    (return 0)
    (else
      (return (Utilities|Array|Get(acopy) _tilesqueue (Utilities|Array|LastIndex _tilesqueue))))))

(fn AddTiletoQueue
  (params (tileRef :type Tile%20Object%20Reference))
  (Utilities|Array|AddUnique (Variables|Default|GettilesQueue) tileRef)
  (Default|SelectTile tileRef))

(fn IsPenultTile
  (params (tileRef :type Tile%20Object%20Reference))
  (return (== tileRef (SpecificTiles|GetPenultTile))))

(fn GetPenultTile
  (bind _tilesqueue (Variables|Default|GettilesQueue))
  (if (>= (Utilities|Array|Length (Variables|Default|GettilesQueue)) 2)
    (return (Utilities|Array|Get(acopy) _tilesqueue (- (Utilities|Array|LastIndex _tilesqueue) 1)))))

(fn MoveCharactertoPosition
  (if (not (Utility|IsQueueEmpty))
    (bind _output_get (Variables|Default|SetcurrentTile (SpecificTiles|GetLastTile)))
    (Transformation|SetActorLocation (Game|Player|GetPlayerPawn 0) (Transformation|GetActorLocation _output_get) false false)
    (if (Utilities|Array|ContainsItem (Variables|Default|GettilesQueue) (Variables|/Game/Blueprints/Field/Field.Field_C|GetfinishTile (Variables|Default|GetfieldRef)))
      (Game|QuitGame 0 "Quit" false))))