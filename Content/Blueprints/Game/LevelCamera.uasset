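; LevelCamera is a camera actor that becomes player 0's view target when play begins.
; Q and E rotate its spring arm in opposite fixed world-space steps, snapping instantly without interpolation.
; BeginPlay also enables input on the actor and adds a TestWidget to the viewport, a block marked TODO for deletion.
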(event EventBeginPlay
  (bind _returnvalue (Game|GetPlayerController 0))
  (Game|Player|SetViewTargetwithBlend _returnvalue self 0.0 "VTBlend_Linear" 0.0 false)
  ;[1 1 1] TODO: DELETE
  (Input|EnableInput _returnvalue)
  (bind _returnvalue_2 (UserInterface|CreateWidget "/Game/Blueprints/Debug/TestWidget.TestWidget_C"))
  (UserInterface|Viewport|AddtoViewport _returnvalue_2 0))

(event Input|KeyboardEvents|Q
  (params (Key :type Key%20Structure))
  ;[1 1 1] TODO: DELETE
  (:Pressed
    (Transformation|AddWorldRotation (Variables|Default|GetSpringArm) "0,30.000000, 0" false false)))

(event Input|KeyboardEvents|E
  (params (Key :type Key%20Structure))
  ;[1 1 1] TODO: DELETE
  (:Pressed
    (Transformation|AddWorldRotation (Variables|Default|GetSpringArm) "0,-30.000000, 0" false false)))

(fn ConstructionScript)