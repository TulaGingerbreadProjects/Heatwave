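; Player character for Heatwave that travels across tiles by following a queue of tiles, starting snapped to the player state's current tile.
; A timeline lerps between tile centers, offset by capsule half-height, with a temporary vertical hop curve marked for removal.
; Each finished move pops the tile and starts the next, clearing the controller's queue when empty.
; It can also snap straight to the queue's last tile.
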(event Custom|initTimeline
  (bind (_direction _alpha _zjumps) (Timeline|movementTimeline SetNewTime)
    (:Update
      (Transformation|SetActorLocation (+ (Math|Vector|Lerp(Vector) (Variables|Movement|GetstartLocation) (Variables|Movement|GetendLocation) _alpha) (Math|Vector|Lerp(Vector) "0, 0, 0" "0, 0,75.000000" _zjumps)) false false))
    (:Finished
      (Movement|FinishMovement))))

(event EventBeginPlay
  (bind _asheatwave_player_controller (Utilities|Casting|CastToHeatwavePlayerController (Game|GetPlayerController 0)))
  (Variables|References|SetcontrollerRef _asheatwave_player_controller)
  (bind _asheatwave_player_state (Utilities|Casting|CastToHeatwavePlayerState (Variables|GetPlayerState)))
  (Variables|References|SetPlayerStateRef _asheatwave_player_state)
  (Movement|SnaptoTile (Variables|/Game/Blueprints/Player/HeatwavePlayerState.HeatwavePlayerState_C|GetcurrentTile (Variables|References|GetPlayerStateRef))))

(fn ConstructionScript)

(fn SnaptoTile
  (params (TileRef :type Tile%20Object%20Reference))
  (Audio|Components|Audio|Stop (Variables|Default|GetmovementTimeline))
  (Transformation|SetActorLocation (+ (Transformation|GetActorLocation TileRef) (Math|Vector|MakeVector 0.0 0.0 (Variables|/Script/Engine.CapsuleComponent|GetCapsuleHalfHeight (Variables|Collision|GetCapsuleComponent)))) false false))

(fn MovetoTile
  (params (tileRef :type Tile%20Object%20Reference))
  (Variables|Movement|SetstartLocation (Transformation|GetActorLocation))
  (Variables|Movement|SetendLocation (+ (Transformation|GetActorLocation tileRef) (Math|Vector|MakeVector 0.0 0.0 (Variables|/Script/Engine.CapsuleComponent|GetCapsuleHalfHeight (Variables|Collision|GetCapsuleComponent)))))
  (Components|Timeline|PlayfromStart (Variables|Default|GetmovementTimeline)))

(fn MoveAlongtheQueue
  (params (startQueue :type Array%20of%20Tile%20Object%20References))
  (bind _output_get (Variables|Movement|Setqueue startQueue))
  (if (!= (Utilities|Array|Length _output_get) 0)
    (Variables|Movement|SetisMoving true)
    (bind _output_get_2 (Variables|Movement|SettargetTile (Utilities|Array|Get(acopy) (Variables|Movement|Getqueue))))
    (Movement|MovetoTile _output_get_2)
    (else
      (Variables|Movement|SetisMoving false)
      (Default|ClearQueue (Variables|References|GetcontrollerRef)))))

(fn FinishMovement
  (Utilities|Array|RemoveItem (Variables|Movement|Getqueue) (Variables|Movement|GettargetTile))
  (Movement|MoveAlongtheQueue (Variables|Movement|Getqueue)))

(fn SnaptoQueueEnd
  (bind _queue (Variables|Movement|Getqueue))
  (Variables|Movement|SetisMoving false)
  (Movement|SnaptoTile (Utilities|Array|Get(acopy) _queue (Utilities|Array|LastIndex _queue)))
  (Default|ClearQueue (Variables|References|GetcontrollerRef)))