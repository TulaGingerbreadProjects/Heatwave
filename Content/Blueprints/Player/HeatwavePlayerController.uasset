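; Player controller for Heatwave that lets the player draw a movement path of tiles while the select input is held.
; Tiles join the queue only if they neighbor the last queued tile or current tile; returning to the second-to-last tile removes the last one.
; Executing the queue updates the player state's tile and moves the character along it, or snaps to the end if already moving.
; A temporary debug widget's start button follows queue state.
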(event EventBeginPlay
  (References|LinkPlayerController)
  (References|LinkPlayerState)
  (References|LinkField)
  (Debug|CreateDebugWidget) ; TODO: delete DEBUG
)

(event Input|ActionEvents|InputActionSelectTile
  (params (Key :type Key%20Structure))
  (:Pressed
    (Variables|Queue|SetisSelecting true))
  (:Released
    (Variables|Queue|SetisSelecting false)
    (Debug|DebugEnableStartQueueButton) ; TODO: delete DEBUG
  ))

(fn ConstructionScript)

(fn AddNeighborTile
  (params (tileRef :type Tile%20Object%20Reference))
  (if (Default|IsNeighbor tileRef (select (Queue|IsQueueEmpty) (Variables|/Game/Blueprints/Player/HeatwavePlayerState.HeatwavePlayerState_C|GetcurrentTile (Variables|References|GetplayerStateRef)) (SpecificTiles|GetLastTile)))
    (ProceedTile|Add|AddTiletoQueue tileRef)))

(fn ClearQueue
  ;[0 0.5 0] Perfect
  (for _array_element (Variables|Queue|GettilesQueue)
    (Default|RemoveTilefromQueue _array_element))
  (Utilities|Array|Clear (Variables|Queue|GettilesQueue)))

(fn ProceedSelectedTile
  (params (tileRef :type Tile%20Object%20Reference))
  ;[0 0.5 0] Perfect
  (if (Variables|Queue|GetisSelecting)
    (if (Default|IsSelected tileRef)
      (ProceedTile|Remove|RemoveifStepBack tileRef)
      (else
        (ProceedTile|Add|AddNeighborTile tileRef)))))

(fn IsLastTile
  (params (tileRef :type Tile%20Object%20Reference))
  ;[0 0.5 0] Perfect
  (return (== tileRef (SpecificTiles|GetLastTile))))

(fn RemoveTilefromQueue
  (params (tileRef :type Tile%20Object%20Reference))
  ;[0 0.5 0] PERFECT
  (Utilities|Array|RemoveItem (Variables|Queue|GettilesQueue) tileRef)
  (Default|RemoveTilefromQueue tileRef))

(fn RemoveifStepBack
  (params (tileRef :type Tile%20Object%20Reference))
  ;[0 0.5 0] Perfect
  (if (SpecificTiles|IsPenultTile tileRef)
    (ProceedTile|Remove|RemoveTilefromQueue (SpecificTiles|GetLastTile))))

(fn IsQueueEmpty
  ;[0 0.5 0] Perfect
  (return (== (Utilities|Array|Length (Variables|Queue|GettilesQueue)) 0)))

(fn GetLastTile
  (bind _tilesqueue (Variables|Queue|GettilesQueue))
  ;[0 0.5 0] Perfect
  (if (Queue|IsQueueEmpty)
    (return 0)
    (else
      (return (Utilities|Array|Get(acopy) _tilesqueue (Utilities|Array|LastIndex _tilesqueue))))))

(fn AddTiletoQueue
  (params (tileRef :type Tile%20Object%20Reference))
  ;[0 0.5 0] Perfect
  (Utilities|Array|AddUnique (Variables|Queue|GettilesQueue) tileRef)
  (Default|SelectTile tileRef))

(fn IsPenultTile
  (params (tileRef :type Tile%20Object%20Reference))
  ;[0 0.5 0] Perfect
  (return (== tileRef (SpecificTiles|GetPenultTile))))

(fn GetPenultTile
  (bind _tilesqueue (Variables|Queue|GettilesQueue))
  ;[0 0.5 0] Perfect
  (if (>= (Utilities|Array|Length (Variables|Queue|GettilesQueue)) 2)
    (return (Utilities|Array|Get(acopy) _tilesqueue (- (Utilities|Array|LastIndex _tilesqueue) 1)))))

(fn ExcecuteQueue
  ;[1 1 1] TODO: REFACTOR; MOVE QUEUE TO CHARACTER
  (if (Variables|/Game/Blueprints/Player/HeatwaveCharacter.HeatwaveCharacter_C|GetisMoving (Variables|References|GetcharacterRef))
    (Default|SnaptoQueueEnd (Variables|References|GetcharacterRef))
    (else
      ;;[1 1 1] TODO: USE IS EMPTY?
      (if (not (Queue|IsQueueEmpty))
        ;[1 1 1] TODO: Edit in character while moving
        (Variables|/Game/Blueprints/Player/HeatwavePlayerState.HeatwavePlayerState_C|SetcurrentTile (Variables|References|GetplayerStateRef) (SpecificTiles|GetLastTile))
        (Default|MoveAlongtheQueue (Variables|References|GetcharacterRef) (Variables|Queue|GettilesQueue))))))

(fn DebugEnableStartQueueButton
  (Widget|SetIsEnabled (Variables|/Game/Blueprints/Debug/TestWidget.TestWidget_C|GetStartQueueButton (Variables|Debug|GetdebugWidgetRef)) (not (Queue|IsQueueEmpty))))

(fn LinkPlayerController
  ;[0 0.5 0] Perfect
  (bind _asheatwave_character (Utilities|Casting|CastToHeatwaveCharacter (Game|Player|GetPlayerPawn 0)))
  (Variables|References|SetcharacterRef _asheatwave_character))

(fn LinkPlayerState
  ;[0 0.5 0] Perfect
  (bind _asheatwave_player_state (Utilities|Casting|CastToHeatwavePlayerState (Variables|GetPlayerState)))
  (Variables|References|SetplayerStateRef _asheatwave_player_state))

(fn CreateDebugWidget
  (bind _returnvalue (UserInterface|CreateWidget "/Game/Blueprints/Debug/TestWidget.TestWidget_C"))
  (bind _output_get (Variables|Debug|SetdebugWidgetRef _returnvalue))
  (UserInterface|Viewport|AddtoViewport _output_get 0))

(fn LinkField
  (bind _asheatwave_game_state (Utilities|Casting|CastToHeatwaveGameState (Game|GetGameState)))
  (Variables|References|SetfieldRef (Default|GetField _asheatwave_game_state)))