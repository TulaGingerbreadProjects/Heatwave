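; ShadowItem is an item actor whose mesh is sized from Length, Width and Height values.
; Its construction script uses the three values as the world scale of ItemMesh.
; It then sets the actor's relative location to that size vector times half of ItemSize, offsetting it by half its extent.
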(fn ConstructionScript
  (bind _length (Variables|Default|Getlength))
  (bind _width (Variables|Default|Getwidth))
  (bind _height (Variables|Default|Getheight))
  (bind _returnvalue (Math|Conversions|ToFloat(Integer) _length))
  (bind _returnvalue_2 (Math|Conversions|ToFloat(Integer) _width))
  (bind _returnvalue_3 (Math|Conversions|ToFloat(Integer) _height))
  (bind _returnvalue_4 (Math|Vector|MakeVector _returnvalue _returnvalue_2 _returnvalue_3))
  (Transformation|SetWorldScale3D (Variables|Default|GetItemMesh) _returnvalue_4)
  (Transformation|SetActorRelativeLocation (* _returnvalue_4 (/ (Variables|Default|GetitemSize) 2))))