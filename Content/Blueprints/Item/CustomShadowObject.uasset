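; CustomShadowObject is a placeable grid object built from cube meshes that casts shade onto field tiles.
; The construction script spawns one cube per ShadowMeshPositions entry, scaled by ObjectSize and shifted by Offset.
; On BeginPlay, each cube shades tiles found through FieldRef, offset from TileRef along Direction by its height and one level below.
; Rotate functions yaw the actor 90 degrees without recomputing shade.
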(event EventBeginPlay
  (Shadow|ShadeTiles))

(fn ConstructionScript
  (bind _objectsize (Variables|ObjectInfo|GetobjectSize))
  (bind (_x _y _z) (Math|Vector|BreakVector _objectsize))
  (for _array_element (Variables|Default|GetshadowMeshPositions)
    (bind _returnvalue (AddComponent|AddStaticMeshComponent false (Math|Conversions|ToTransform(Vector) (+ (Math|Vector|MakeVector (* (.length (Utilities|Struct|BreakPosition _array_element)) _x) (* (.width (Utilities|Struct|BreakPosition _array_element)) _y) (* (.height (Utilities|Struct|BreakPosition _array_element)) _z)) (LocalVariables|Getoffset)))))
    (Components|StaticMesh|SetStaticMesh _returnvalue "/Game/Assets/Meshes/TestCube.TestCube")
    (Rendering|Material|SetMaterial _returnvalue 0 "/Game/Assets/Materials/Test_M.Test_M")
    (Utilities|Array|Add (Variables|Default|GetshadowMeshComponents) _returnvalue)))

(fn RotateLeft
  (Class|Actor|AddActorWorldRotation "0,-90.000000, 0"))

(fn RotateRight
  (Class|Actor|AddActorWorldRotation "0,90.000000, 0"))

(fn ShadeTiles
  (for _array_element (Variables|Default|GetshadowMeshPositions)
    (CallFunction|ShadeTilebyMeshat _array_element)
    (CallFunction|ShadeTilebyMeshat (Utilities|Struct|MakePosition (.length (Utilities|Struct|BreakPosition _array_element)) (.width (Utilities|Struct|BreakPosition _array_element)) (- (.height (Utilities|Struct|BreakPosition _array_element)) 1)))))

(fn GetShadowDirection
  (return (Variables|Default|Getdirection)))

(fn GetShadowIndex
  (params (length :type Integer) (width :type Integer) (height :type Integer))
  (bind _returnvalue (+ height 1))
  (bind _returnvalue_2 (+ height 1))
  (return (+ (Variables|/Game/Blueprints/Field/Tile.Tile_C|Getrow (Variables|References|GettileRef)) length (Utilities|Select :Index (Shadow|GetShadowDirection) :NewEnumerator0 _returnvalue_2 :NewEnumerator1 0 :NewEnumerator2 (* _returnvalue_2 -1) :NewEnumerator3 0)) (+ (Variables|/Game/Blueprints/Field/Tile.Tile_C|Getcolumn (Variables|References|GettileRef)) width (Utilities|Select :Index (Shadow|GetShadowDirection) :NewEnumerator0 0 :NewEnumerator1 _returnvalue :NewEnumerator2 0 :NewEnumerator3 (* _returnvalue -1)))))

(fn ShadeTilebyMeshat
  (params (Position :type Position%20Structure%20%28by%20ref%29))
  (bind (_length _width _height) (Utilities|Struct|BreakPosition Position))
  (bind (_rowindex _columnindex) (Shadow|GetShadowIndex _length _width _height))
  (LocalVariables|SetshadowStartRow _rowindex)
  (LocalVariables|SetshadowStartColumn _columnindex)
  (bind _tileref (Default|GetTileat (Variables|References|GetfieldRef) (LocalVariables|GetshadowStartRow) (LocalVariables|GetshadowStartColumn)))
  (Utilities|IsValid _tileref
    (:Is%20Valid
      (Default|ShadeTile _tileref)
      (Development|PrintString (Utilities|String|Append "Shaded tile at row " (Utilities|String|ToString(Integer) (LocalVariables|GetshadowStartRow)) "; column " (Utilities|String|ToString(Integer) (LocalVariables|GetshadowStartColumn))) true true "(R=0.000000,G=0.660000,B=1.000000,A=1.000000)" 2e+01))))