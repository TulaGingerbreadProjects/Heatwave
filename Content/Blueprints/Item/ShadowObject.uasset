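; ShadowObject is a grid-placed, rotatable object that shades and locks field tiles around it.
; Construction builds mesh blocks from a list of length, width and height positions, with toggleable visibility.
; Tile indices come from TileRef plus rotation-aware offsets, with shadows projected further by height along a stored cardinal light direction.
; Shortly after BeginPlay, and on UpdateTiles, it shades projected tiles and locks tiles under low blocks.
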(event EventBeginPlay
  (Utilities|FlowControl|Delay 0.2) ; Time to re-link all tiles
  (Shadow|ShadeTiles)
  (Manage|LockTiles))

(fn ConstructionScript
  ;[1 1 1] TODO: extract to function?
  (for _array_element (Variables|ShadowMesh|GetshadowMeshPositions)
    (bind _returnvalue (AddComponent|AddStaticMeshComponent false (|getMeshTransform _array_element)))
    (Utilities|Array|Add (Variables|ShadowMesh|GetshadowMeshComponents) _returnvalue))
  (Shadow|ShadowMesh|SetShadowMeshVisibility (Variables|ShadowMesh|GetisMeshVisible)))

(fn RotateLeft
  ;[0 0.5 0] Perfect
  (Class|Actor|AddActorWorldRotation "0,-90.000000, 0"))

(fn RotateRight
  ;[0 0.5 0] Perfect
  (Class|Actor|AddActorWorldRotation "0,90.000000, 0"))

(fn ShadeTiles
  ;[0 0.5 0] Perfect
  (for _array_element (Variables|ShadowMesh|GetshadowMeshPositions)
    (Shadow|ShadeTilebyMeshat _array_element)
    (Shadow|ShadeTilebyMeshat (Utilities|Struct|MakePosition (.length (Utilities|Struct|BreakPosition _array_element)) (.width (Utilities|Struct|BreakPosition _array_element)) (- (.height (Utilities|Struct|BreakPosition _array_element)) 1)))))

(fn GetLightDirection
  ;[1 1 1] TODO: USE SUN LIGHT DIRECTION
  (return (Variables|Shadow|GetlightDirection)))

(fn GetTileIndexShadedbyMesh
  (params (position :type Position%20Structure))
  (bind (_row _column) (Index|GetTileIndexUnderMesh position))
  ;[0 0.5 0] Perfect
  (LocalVariables|Setheight (.height (Utilities|Struct|BreakPosition position)))
  (return (+ (Index|GetRowHeightOffset (LocalVariables|Getheight)) _row) (+ _column (Index|GetColumnHeightOffset (LocalVariables|Getheight)))))

(fn ShadeTilebyMeshat
  (params (Position :type Position%20Structure%20%28by%20ref%29))
  ;[0 0.5 0] Perfect
  (bind (_rowindex _columnindex) (Index|GetTileIndexShadedbyMesh Position))
  (LocalVariables|SetshadowRowIndex _rowindex)
  (LocalVariables|SetshadowColumnIndex _columnindex)
  (bind _tileref (Default|GetTileat (Variables|References|GetfieldRef) (LocalVariables|GetshadowRowIndex) (LocalVariables|GetshadowColumnIndex)))
  (Utilities|IsValid _tileref
    (:Is%20Valid
      (Default|ShadeTile _tileref)
      (Development|PrintString (Utilities|String|Append "Shaded tile at row " (Utilities|String|ToString(Integer) (LocalVariables|GetshadowRowIndex)) "; column " (Utilities|String|ToString(Integer) (LocalVariables|GetshadowColumnIndex))) false true "(R=0.000000,G=0.660000,B=1.000000,A=1.000000)" 2e+01))))

(fn SetShadowMeshVisibility
  (params (newVisibility :type Boolean))
  ;[0 0.5 0] Perfect
  (Variables|ShadowMesh|SetisMeshVisible newVisibility)
  (for _array_element (Variables|ShadowMesh|GetshadowMeshComponents)
    (Rendering|SetVisibility _array_element (Variables|ShadowMesh|GetisMeshVisible) false)))

(fn GetRotationDirection
  ;[1 1 1] TODO: CreateFuncLibrary?
  (return (Utilities|Enum|ByteToEnumDirection (Class|KismetMathLibrary|PercentByteByte (Math|Conversions|ToByte(Integer) (/ (Math|Float|Round (+ (.Yaw (Math|Rotator|BreakRotator (Transformation|GetActorRotation))) 3.6e+02)) 90)) 4))))

(fn LockTiles
  ;[0 0.5 0] Perfect
  (for _array_element (Variables|ShadowMesh|GetshadowMeshPositions)
    (if (< (.height (Utilities|Struct|BreakPosition _array_element)) 2)
      (bind _tileref (Default|GetTileat (Variables|References|GetfieldRef) (.row (Index|GetTileIndexUnderMesh _array_element)) (.column (Index|GetTileIndexUnderMesh _array_element))))
      (Utilities|IsValid _tileref
        (:Is%20Valid
          (Default|LockTile _tileref))))))

(fn GetTileIndexUnderMesh
  (params (position :type Position%20Structure))
  (bind (_length _width) (Utilities|Struct|BreakPosition position))
  ;[0 0.5 0] Perfect
  (LocalVariables|Setlength _length)
  (LocalVariables|Setwidth _width)
  (return (+ (Variables|/Game/Blueprints/Field/Tile.Tile_C|Getrow (Variables|References|GettileRef)) (Index|GetRowOffset (LocalVariables|Getlength) (LocalVariables|Getwidth))) (+ (Variables|/Game/Blueprints/Field/Tile.Tile_C|Getcolumn (Variables|References|GettileRef)) (Index|GetColumnOffset (LocalVariables|Getlength) (LocalVariables|Getwidth)))))

(fn GetRowOffset
  (params (length :type Integer) (width :type Integer))
  ;[0 0.5 0] Perfect
  (return (Utilities|Select :Index (Direction|GetRotationDirection) :NewEnumerator0 length :NewEnumerator1 (* width -1) :NewEnumerator2 (* length -1) :NewEnumerator3 width)))

(fn GetColumnOffset
  (params (length :type Integer) (width :type Integer))
  ;[0 0.5 0] Perfect
  (return (Utilities|Select :Index (Direction|GetRotationDirection) :NewEnumerator0 width :NewEnumerator1 length :NewEnumerator2 (* width -1) :NewEnumerator3 (* length -1))))

(fn UpdateTiles
  ;[0 0.5 0] Perfect
  (Shadow|ShadeTiles)
  (Manage|LockTiles))

(fn GetRowHeightOffset
  (params (height :type Integer))
  (bind _returnvalue (+ height 1))
  ;[0 0.5 0] Perfect
  (return (Utilities|Select :Index (Direction|GetLightDirection) :NewEnumerator0 _returnvalue :NewEnumerator1 0 :NewEnumerator2 (* _returnvalue -1) :NewEnumerator3 0)))

(fn GetColumnHeightOffset
  (params (height :type Integer))
  (bind _returnvalue (+ height 1))
  ;[0 0.5 0] Perfect
  (return (Utilities|Select :Index (Direction|GetLightDirection) :NewEnumerator0 0 :NewEnumerator1 _returnvalue :NewEnumerator2 0 :NewEnumerator3 (* _returnvalue -1))))