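; Blueprint function library for working with a four-value Direction enum.
; IncreaseDirection and DecreaseDirection step one value forward or back with modulo-4 wraparound, adding 3 to go backwards.
; ConvertRotationToDirecton maps a rotator's yaw to a Direction by adding 360, rounding, dividing by 90 and wrapping modulo 4.
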(fn IncreaseDirection
  (params (startDirection :type Direction%20Enum :default "NewEnumerator0"))
  (return (Utilities|Enum|ByteToEnumDirection (Class|KismetMathLibrary|PercentByteByte (+ startDirection 1) 4))))

(fn DecreaseDirection
  (params (startDirection :type Byte))
  (return (Utilities|Enum|ByteToEnumDirection (Class|KismetMathLibrary|PercentByteByte (+ startDirection 3) 4))))

(fn ConvertRotationtoDirecton
  (params (rotator :type Rotator))
  (return (Utilities|Enum|ByteToEnumDirection (Class|KismetMathLibrary|PercentByteByte (Math|Conversions|ToByte(Integer) (/ (Math|Float|Round (+ (.Yaw (Math|Rotator|BreakRotator rotator)) 3.6e+02)) 90)) 4))))