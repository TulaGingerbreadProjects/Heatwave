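; Blueprint function library that converts between chapter and level indexes and level names.
; GetLevelNameFromIndex builds a Name in the "Level<Chapter>_<Level>" pattern from the two indexes.
; GetIndexesFromLevelName reverses this by removing the "Level" prefix, splitting on the underscore and converting both halves to integers.
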(fn GetLevelNamefromIndex
  (params (chapter :type Integer) (level :type Integer))
  (return (Utilities|String|StringToName (Utilities|String|Append "Level" (Utilities|String|ToString(Integer) chapter) "_" (Utilities|String|ToString(Integer) level)))))

(fn GetIndexesfromLevelName
  (params (levelName :type String))
  (bind _returnvalue (Utilities|String|Replace levelName "Level"))
  (bind (_lefts _rights) (Utilities|String|Split _returnvalue "_"))
  (return (Math|Conversions|ToInteger(Byte) _lefts) (Math|Conversions|ToInteger(Byte) _rights)))