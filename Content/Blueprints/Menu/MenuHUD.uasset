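; MenuHUD is a menu controller that routes menu commands to main, level selection, settings, pause and exit handlers.
; OpenMenu guards against re-entry with IsOpening, calls CloseAllMenues, stores the command, fires OnStartOpening, then switches on menu type.
; The handler's result is written back to IsOpening.
; Menu opening is stubbed with debug prints and closing is empty; only Exit acts, quitting the game.
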(fn ConstructionScript)

(fn OpenMenu
  (params (menuCommand :type Menu%20Command%20Object%20Reference))
  (if (not (Variables|Default|GetisOpening))
    (Variables|Default|SetisOpening true)
    (Menu|CloseAllMenues)
    (Variables|Default|SetcurrentMenu menuCommand)
    (Default|CallOnStartOpening (Variables|Default|GetcurrentMenu))
    (switch Utilities|FlowControl|Switch|SwitchonMenuType (Variables|/Game/Blueprints/Objects/menuCommand.menuCommand_C|GetmenuType (Variables|Default|GetcurrentMenu))
      (:NewEnumerator4
        (bind _isopened (Menu|OpenMainMenu))
        (LocalVariables|Setlocal_isOpened _isopened))
      (:NewEnumerator0
        (bind _isopened_2 (Menu|OpenLevels))
        (LocalVariables|Setlocal_isOpened _isopened_2))
      (:NewEnumerator1
        (bind _isopened_3 (Menu|OpenSettings))
        (LocalVariables|Setlocal_isOpened _isopened_3))
      (:NewEnumerator5
        (bind _isopened_4 (Menu|OpenPauseMenu))
        (LocalVariables|Setlocal_isOpened _isopened_4))
      (:NewEnumerator2
        (bind _isopened_5 (Menu|Exit))
        (LocalVariables|Setlocal_isOpened _isopened_5)))
    (bind _output_get (Variables|Default|SetisOpening (LocalVariables|Getlocal_isOpened)))
    (return _output_get)))

(fn OpenSettings
  (Development|PrintString "Open settings menu"))

(fn OpenLevels
  (Development|PrintString "Open level selection menu"))

(fn Exit
  (Development|PrintString "Quit game")
  (Game|QuitGame 0 "Quit" false))

(fn OpenPauseMenu
  (Development|PrintString "Open pause menu"))

(fn OpenMainMenu
  (Development|PrintString "Open main menu")
  (return false))

(fn CloseAllMenues)