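; Main menu HUD that switches between the main screen and submenus hosted on Stella actors in the level.
; OpenMenu opens the Stella owning the menu command, or returns through a Back widget, closing its Stella and signalling the player pawn as view target.
; An IsOpening flag blocks new requests until the animation-finished event clears it and announces the current menu.
; BeginPlay caches every Stella for event binding and bulk closing.
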(event Custom|onOpenAnimationFinished
  (Variables|Default|SetisOpening false)
  (Default|CallOnOpened (Variables|Default|GetcurrentMenu)))

(event EventOpenMainMenu
  (params (menuCommand :type Menu%20Command%20Object%20Reference))
  (bind _asback_w (Utilities|Casting|CastToBack_W (Utilities|GetOuterObject menuCommand)))
  (Default|CloseStellaMenu (Variables|/Game/Blueprints/Menu/UMG/Back_W.Back_W_C|GetStellaRef _asback_w))
  (Default|CallOnStartOpening (Game|Player|GetPlayerPawn 0)))

(event EventBeginPlay
  (bind _outactors (Actor|GetAllActorsOfClass "/Game/Blueprints/Menu/Stella/Stella.Stella_C"))
  (bind _output_get (Variables|Default|SetmenuStellas _outactors))
  (for _array_element _output_get
    (EventDispatchers|BindEventtoOnStellaMenuOpened _array_element (EventDispatchers|CreateEvent :!event Custom|onOpenAnimationFinished))))

(fn ConstructionScript
  (|CallParentFunction))

(fn OpenMenu
  (params (menuCommand :type Menu%20Command%20Object%20Reference))
  ;[1 1 1] TODO: fix hardcode?
  (if (not (Variables|Default|GetisOpening))
    (Variables|Default|SetisOpening true)
    (Variables|Default|SetcurrentMenu (Variables|/Game/Blueprints/Objects/menuCommand.menuCommand_C|GetmenuType menuCommand))
    (bind _asstella (Utilities|Casting|CastToStella (Utilities|GetOuterObject menuCommand))
      (:then
        (Default|OpenStellaMenu _asstella)
        (Default|CallOnStartOpening _asstella))
      (:CastFailed
        (CallFunction|OpenMainMenu menuCommand)))
    (return false)))

(fn CloseAllMenues
  (for _array_element (Variables|Default|GetmenuStellas)
    (Default|CloseStellaMenu _array_element)))