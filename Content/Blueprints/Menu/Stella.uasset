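; Stella is a clickable 3D main menu actor that acts as Choose Level, Settings or Exit, based on StellaType.
; Cursor hover swaps its mesh between cold and hot materials.
; Choose Level and Settings play a timeline that moves the mesh vertically, blends the camera to this actor, disables mouse-over events and reveals a widget after a delay.
; Exit runs the console exit command.
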(event MouseInput|EventActorOnClicked
  (params (ButtonPressed :type Key%20Structure))
  (switch Utilities|FlowControl|Switch|SwitchonMenuButtons (Variables|Default|GetStellaType)
    (:NewEnumerator0
      (bind _alpha (Timeline|StellaLocationAlpha Play)
        (:Update
          (CallFunction|SwitchtoSubMenu _alpha)
          (Utilities|FlowControl|Delay 2.1)
          (Rendering|SetVisibility (Variables|Default|GetWidget) true false))))
    (:NewEnumerator1
      (Timeline|StellaLocationAlpha Play))
    (:NewEnumerator2
      (Development|ExecuteConsoleCommand "Exit" 0))))

(event MouseInput|EventActorBeginCursorOver
  (Rendering|Material|SetMaterial (Variables|Default|GetStaticMesh) 0 (Variables|Materials|GetColdMaterial)))

(event MouseInput|EventActorEndCursorOver
  (Rendering|Material|SetMaterial (Variables|Default|GetStaticMesh) 0 (Variables|Materials|GetHotMaterial)))

(event EventBeginPlay
  (bind _asmenu_player_controller (Utilities|Casting|CastToMenuPlayerController (Game|GetPlayerController 0)))
  (Variables|Default|SetPC_Ref _asmenu_player_controller))

(fn ConstructionScript)

(fn SwitchtoSubMenu
  (params (Alpha :type Float%20%28single-precision%29))
  ;[1 1 1] Move Stella
  (Transformation|SetRelativeLocation (Variables|Default|GetStaticMesh) (Math|Vector|MakeVector 0.0 0.0 (Math|Float|Lerp -2e+02 4e+02 Alpha)) false false)
  ;[1 1 1] Switch Camera
  (Game|Player|SetViewTargetwithBlend (Variables|Default|GetPC_Ref) self 2.0 "VTBlend_Linear" 0.0 false)
  ;[1 1 1] Disable Mouse Over Events
  (Variables|/Script/Engine.PlayerController|SetbEnableMouseOverEvents (Variables|Default|GetPC_Ref) false))