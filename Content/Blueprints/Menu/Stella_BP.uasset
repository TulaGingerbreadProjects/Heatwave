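; Stella_BP is a clickable static mesh actor in the Menu folder that stretches vertically when clicked.
; A click plays the StellaScaleAlpha timeline from the start, lerping the mesh's relative Z scale from its base to a taller size.
; Cursor hover events only print debug strings, and the hot and cold material swaps are left unconnected.
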(event MouseInput|EventActorOnClicked
  (params (ButtonPressed :type Key%20Structure))
  (bind _alpha (Timeline|StellaScaleAlpha PlayFromStart)
    (:Update
      (Transformation|SetRelativeScale3D (Variables|Debug|GetStaticMeshComponent) (Math|Vector|MakeVector 1.0 1.0 (Math|Float|Lerp 1.0 6.0 _alpha))))))

(event MouseInput|EventActorBeginCursorOver
  (Development|PrintString "Hovered"))

(event MouseInput|EventActorEndCursorOver
  (Development|PrintString "Not Hovered"))

(fn ConstructionScript)