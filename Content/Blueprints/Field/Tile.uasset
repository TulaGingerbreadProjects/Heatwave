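; Field tile Blueprint with editor events for building out a tile grid from an existing tile.
; Directional events append a neighbor by offsetting Row and Column, and the tile can also remove itself; both go through FieldRef.
; AppendGrid fills a GridRows by GridColumns block starting at this tile, with GetBounds using each count's sign to set the direction it extends.
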(event Custom|AppendTileLeft
  (AddTiles|AppendTileto "NewEnumerator3"))

(event Custom|AppendTileAbove
  (AddTiles|AppendTileto "NewEnumerator0"))

(event Custom|AppendTileRight
  (AddTiles|AppendTileto "NewEnumerator1"))

(event Custom|AppendTileBelow
  (AddTiles|AppendTileto "NewEnumerator2"))

(fn ConstructionScript)

(fn AppendTileto
  (params (direction :type Direction%20Enum :default "NewEnumerator0"))
  (Default|AddTileat (Variables|References|GetfieldRef) (+ (Variables|TileInfo|Getrow) (Utilities|Select :Index direction :NewEnumerator0 0 :NewEnumerator1 1 :NewEnumerator2 0 :NewEnumerator3 -1)) (+ (Variables|TileInfo|Getcolumn) (Utilities|Select :Index direction :NewEnumerator0 1 :NewEnumerator1 0 :NewEnumerator2 -1 :NewEnumerator3 0))))

(fn RemovefromField
  (Default|RemoveTileat (Variables|References|GetfieldRef) (Variables|TileInfo|Getrow) (Variables|TileInfo|Getcolumn)))

(fn AppendGrid
  (bind _row (Variables|TileInfo|Getrow))
  (bind _gridrows (Variables|Grid|GetgridRows))
  (bind _column (Variables|TileInfo|Getcolumn))
  (bind _gridcolumns (Variables|Grid|GetgridColumns))
  (bind (_min _max) (CallFunction|GetBounds _row _gridrows))
  (bind (_min_2 _max_2) (CallFunction|GetBounds _column _gridcolumns))
  (for _index (range _min _max)
    (LocalVariables|SetrowIndex _index)
    (for _index_2 (range _min_2 _max_2)
      (LocalVariables|SetcolumnIndex _index_2)
      (Default|AddTileat (Variables|References|GetfieldRef) (LocalVariables|GetrowIndex) (LocalVariables|GetcolumnIndex)))))

(fn GetBounds
  (params (dimention :type Integer) (offset :type Integer))
  (bind _returnvalue (Class|KismetMathLibrary|SignOfInteger offset))
  (bind _returnvalue_2 (- offset _returnvalue))
  (bind _returnvalue_3 (+ dimention _returnvalue_2))
  (return (Math|Integer|Min(Integer) dimention _returnvalue_3) (Math|Integer|Max(Integer) dimention _returnvalue_3)))