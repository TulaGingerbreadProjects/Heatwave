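; Field actor that manages a sparse 2D grid of spawned Tile actors, stored as an array of row structs.
; InitField clears the grid and spawns a single starting tile at the start row and column.
; Add and remove functions check tile existence first, growing rows and columns on demand and passing each tile its coordinates and a field reference.
; Tile placement is meant to be relative to the field's location and start cell.
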(fn ConstructionScript)

(fn AddTileat
  (params (row :type Integer) (column :type Integer))
  (bind _isexist (FieldFunctions|IsTileExist row column))
  (if (not _isexist)
    (bind _returnvalue (Game|SpawnActorfromClass "/Game/Blueprints/Field/Tile.Tile_C" (|getTileTransform) "AlwaysSpawn" 0 row column self 0))
    (FieldFunctions|ValidateRow row)
    (Utilities|Array|SetArrayElem (.row (Utilities|Array|Get(acopy) (Variables|Default|Gettiles) row)) column _returnvalue true)))

(fn InitField
  (FieldFunctions|ClearField)
  (CallFunction|AddTileat (Variables|Default|GetstartRow) (Variables|Default|GetstartColumn)))

(fn ClearField
  (for _array_element (Variables|Default|Gettiles)
    (FieldFunctions|ClearRow (.row _array_element)))
  (Utilities|Array|Clear (Variables|Default|Gettiles)))

(fn ClearRow
  (params (row :type Array%20of%20Tile%20Object%20References))
  (for _array_element row
    (Utilities|IsValid _array_element
      (:Is%20Valid
        (Actor|DestroyActor _array_element)))))

(fn ValidateRow
  (params (row :type Integer))
  (if (< row (Utilities|Array|Length (Variables|Default|Gettiles)))
    _
    (else
      (Utilities|Array|SetArrayElem (Variables|Default|Gettiles) row (Utilities|Struct|MakeRowOfTiles (Utilities|Array|MakeArray 0)) true)))
  (return))

(fn IsTileExist
  (params (row :type Integer) (column :type Integer))
  (if (< row (Utilities|Array|Length (Variables|Default|Gettiles)))
    (if (< column (Utilities|Array|Length (.row (Utilities|Array|Get(acopy) (Variables|Default|Gettiles) row))))
      (return (Utilities|IsValid (Utilities|Array|Get(acopy) (.row (Utilities|Array|Get(acopy) (Variables|Default|Gettiles) row)) column)))
      (else
        _)))
  (return false))

(fn RemoveTileat
  (params (row :type Integer) (column :type Integer))
  (bind _isexist (FieldFunctions|IsTileExist row column))
  (if _isexist
    (Actor|DestroyActor (Utilities|Array|Get(acopy) (.row (Utilities|Array|Get(acopy) (Variables|Default|Gettiles) row)) column))))