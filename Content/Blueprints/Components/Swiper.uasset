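; Swiper component that detects four-way swipes from mouse or touch input and reports the direction through OnSwipeCompleted.
; StartSwipe runs a looping timer to accumulate previous-minus-current position deltas until either axis exceeds SwipeLength, then reports and stops.
; Input position sums mouse and chosen-finger touch coordinates rather than selecting a source.
; Direction resolves to an enum value, with X taking priority over Y.
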(fn StartSwipe
  (Variables|Default|Setswipe "")
  (Variables|Position|SetpreviousPosition (Position|GetInputPosition))
  (Variables|Manage|SetbIsSwiping true)
  (bind _returnvalue (Utilities|Time|SetTimerbyEvent (EventDispatchers|CreateEvent :!event UpdateSwipe) 0.1 true))
  (Variables|Manage|SetupdateTimerHandle _returnvalue))

(fn StopSwipe
  (Variables|Manage|SetbIsSwiping false)
  (Utilities|Time|ClearandInvalidateTimerbyHandle (Variables|Manage|GetupdateTimerHandle)))

(fn IsSwipeCompleted
  (return (or (> (Math|Float|Absolute(Float) (.X (Math|Vector2D|BreakVector2D (Variables|Default|Getswipe)))) (Variables|Manage|GetswipeLength)) (> (Math|Float|Absolute(Float) (.Y (Math|Vector2D|BreakVector2D (Variables|Default|Getswipe)))) (Variables|Manage|GetswipeLength)))))

(fn UpdateSwipe
  (Position|IncreaseSwipe)
  (Variables|Position|SetpreviousPosition (Position|GetInputPosition)) ; Important: \nupdate previous position after swipe, \ncoz it used in getSwipeDelta\nOtherwise getSwipeDelta return 0
  (if (Manage|IsSwipeCompleted)
    (Default|CallOnSwipeCompleted (Direction|GetSwipeDirection))
    (Manage|StopSwipe)))

(fn IncreaseSwipe
  (Variables|Default|Setswipe (+ (Variables|Default|Getswipe) (Position|GetSwipeDelta))))

(fn GetSwipeDirection
  (bind _swipe (Variables|Position|GetSwipe))
  (bind (_x _y) (Math|Vector2D|BreakVector2D _swipe))
  (LocalVariables|SetX _x)
  (LocalVariables|SetY _y)
  (if (> (Math|Float|Absolute(Float) (LocalVariables|GetX)) (Variables|Manage|GetswipeLength))
    (if (> (LocalVariables|GetX) 0.0)
      (return "NewEnumerator3")
      (else
        (return "NewEnumerator1")))
    (elif (> (LocalVariables|GetY) 0.0)
      (return "NewEnumerator0")
      (else
        (return "NewEnumerator2")))))

(fn GetSwipeDelta
  (return (- (Variables|Position|GetpreviousPosition) (Position|GetInputPosition))))

(fn GetInputPosition
  (bind _returnvalue (Game|GetPlayerController 0))
  (bind _returnvalue_2 (Game|GetPlayerController 0))
  (bind _swipefingerindex (Variables|Manage|GetswipeFingerIndex))
  (bind (_locationx _locationy) (Class|PlayerController|GetInputTouchState _returnvalue _swipefingerindex))
  (bind (_locationx_2 _locationy_2) (Game|Player|GetMousePosition _returnvalue_2))
  (return (+ (Math|Vector2D|MakeVector2D _locationx_2 _locationy_2) (Math|Vector2D|MakeVector2D _locationx _locationy))))

(fn IsSwiping
  (return (Variables|Manage|GetbIsSwiping)))