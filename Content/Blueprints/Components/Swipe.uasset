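; Swipe component that detects four-directional swipe gestures from mouse or touch input.
; While a swipe is active, a looping timer accumulates position deltas (previous minus current) instead of using Tick.
; Once either axis exceeds SwipeLength, it fires OnSwipeCompleted and stops the timer; GetSwipeDirection maps the vector to an enum, checking X first.
; Input position is the sum of mouse and touch positions, so one path serves both.
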(fn StartSwipe
  (Variables|Default|Setswipe "")
  (Variables|Default|SetpreviousPosition (Position|GetInputPosition))
  (Variables|Default|SetisSwiping true)
  (bind _returnvalue (Utilities|Time|SetTimerbyEvent (EventDispatchers|CreateEvent :!event UpdateSwipe) 0.1 true))
  (Variables|Default|SetupdateTimerHandle _returnvalue))

(fn FinishSwipe
  (Variables|Default|SetisSwiping false)
  (Utilities|Time|ClearandInvalidateTimerbyHandle (Variables|Default|GetupdateTimerHandle)))

(fn IsSwipeCompleted
  (return (or (> (Math|Float|Absolute(Float) (.X (Math|Vector2D|BreakVector2D (Variables|Default|Getswipe)))) (Variables|Default|GetswipeLength)) (> (Math|Float|Absolute(Float) (.Y (Math|Vector2D|BreakVector2D (Variables|Default|Getswipe)))) (Variables|Default|GetswipeLength)))))

(fn UpdateSwipe
  (Position|IncreaseSwipe)
  (Variables|Default|SetpreviousPosition (Position|GetInputPosition)) ; Important: \nupdate previous position after swipe, \ncoz it used in getSwipeDelta\nOtherwise getSwipeDelta return 0
  (if (CallFunction|IsSwipeCompleted)
    (Default|CallOnSwipeCompleted)
    (CallFunction|FinishSwipe)))

(fn IncreaseSwipe
  (Variables|Default|Setswipe (+ (Variables|Default|Getswipe) (Position|GetSwipeDelta))))

(fn GetSwipeDirection
  (bind _swipe (Variables|Default|GetSwipe))
  (bind (_x _y) (Math|Vector2D|BreakVector2D _swipe))
  (LocalVariables|SetX _x)
  (LocalVariables|SetY _y)
  (if (> (Math|Float|Absolute(Float) (LocalVariables|GetX)) (Variables|Default|GetswipeLength))
    (if (> (LocalVariables|GetX) 0.0)
      (return "NewEnumerator3")
      (else
        (return "NewEnumerator1")))
    (elif (> (LocalVariables|GetY) 0.0)
      (return "NewEnumerator0")
      (else
        (return "NewEnumerator2")))))

(fn GetSwipeDelta
  (return (- (Variables|Default|GetpreviousPosition) (Position|GetInputPosition))))

(fn GetInputPosition
  (bind _returnvalue (Game|GetPlayerController 0))
  (bind _returnvalue_2 (Game|GetPlayerController 0))
  (bind _swipefingerindex (Variables|Default|GetswipeFingerIndex))
  (bind (_locationx _locationy) (Class|PlayerController|GetInputTouchState _returnvalue _swipefingerindex))
  (bind (_locationx_2 _locationy_2) (Game|Player|GetMousePosition _returnvalue_2))
  (return (+ (Math|Vector2D|MakeVector2D _locationx_2 _locationy_2) (Math|Vector2D|MakeVector2D _locationx _locationy))))